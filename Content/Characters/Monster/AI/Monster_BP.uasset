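; Monster AI character that detects, chases and attacks the first-person player, with health and ragdoll death.
; PawnSensing sight and noise events raise a clamped threat level and store the player, driving an enum state machine.
; Tick decays evasion and threat through delays, sets speed per state, checks attack range and updates the threat and health widgets.
; Attack and hit states set Monster_AnimBP flags, with damage gated by a resetting DoOnce.
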(event `self.ReceiveBeginPlay`
  ;[1 1 1] Events
  (`self.SetStartingVector`))

(event `self.ReceiveTick`
  (params (DeltaSeconds :type "Float (single-precision)"))
  ;[1 1 1] Events
  (`self.ReduceEvasion`)
  (`self.Reduce Threat Level`)
  (`self.SetSpeedPerState`)
  (`self.SetThreatMeter`)
  (`self.SetThreatMeterVisibility`)
  (`self.CheckPlayerHealth`)
  (`self.SetHealth`)
  (`self.MonsterDeathEvent`)
  (`self.CheckPlayerDist`))

(event `self.PawnSensing.OnSeePawn`
  (params (Pawn :type "Pawn Object Reference"))
  ;[1 1 1] Raise threat level when player is seen
  (switch `/Game/Characters/Monster/AI/Monster_AI_State` (`self.Monster_AI_State`)
    (:`NewEnumerator0`
      _)
    (:`NewEnumerator1`
      _)
    (:`NewEnumerator2`
      _)
    (:`NewEnumerator3`
      _)
    (:`NewEnumerator4`
      _))
  (bind _asfirst_person_character (cast `/Game/FirstPersonBP/Blueprints/FirstPersonCharacter` Pawn))
  (`|ExecutionSequence`
    (:`then_0`
      (set `self.Monster_AI_State` "NewEnumerator1"))
    (:`then_1`
      (set `self.Evasion` 4)
      (bind _output_get (set `self.Player` _asfirst_person_character))
      (bind _returnvalue (`self.K2_GetActorLocation` _output_get))
      (set `self.PlayerVector` _returnvalue)
      (if (< (`KismetMathLibrary.VSize` (- _returnvalue (`self.K2_GetActorLocation`))) 700.0)
        (`self.RaiseThreatLevel` 1.0)
        (else
          (`self.RaiseThreatLevel` 0.25))))
    (:`then_2`
      (if (== (`self.ThreatLevel`) 1.0)
        (set `self.Evasion` 10)
        (set `self.Monster_AI_State` "NewEnumerator2")))))

(event `ReduceEvasion`
  ;[1 1 1] Reduce evasion
  (`KismetSystemLibrary.Delay` 1.0)
  (bind _output_get (set `self.Evasion` (- (`self.Evasion`) 1)))
  (set `self.Evasion` (`KismetMathLibrary.Clamp` _output_get 0 _output_get)))

(event `SetStartingVector`
  ;[1 1 1] Set starting vector
  (set `self.StartingVector` (`self.K2_GetActorLocation`)))

(event `RaiseThreatLevel`
  (params (Value :type "Float (double-precision)"))
  ;[1 1 1] Alter Threat Level
  (bind _output_get (set `self.ThreatLevel` (+ (`self.ThreatLevel`) (+ Value (/ (`self.ThreatLevel`) 20.0)))))
  (set `self.ThreatLevel` (`KismetMathLibrary.FClamp` _output_get)))

(event `Reduce Threat Level`
  ;[1 1 1] Reduce threat level
  (`KismetSystemLibrary.Delay` 0.2)
  (if (`KismetSystemLibrary.IsValid` (`self.Player`))
    (if (== (`self.Evasion`) 0)
      (`self.LowerThreatLevel` 0.025)
      (`|ExecutionSequence`
        (:`then_0`
          (`KismetSystemLibrary.Delay` 2.0)
          (if (== (`self.ThreatLevel`) 0.0)
            (set `self.Monster_AI_State` "NewEnumerator4")))
        (:`then_1`
          (`/Engine/EditorBlueprintResources/StandardMacros.DoOnce` false :!label _label
            (:`Completed`
              (set `self.Monster_AI_State` "NewEnumerator1"))))))))

(event `SetThreatMeter`
  ;[1 1 1] Set Threat Meter percent value
  (bind _asthreat_meter_widget (cast `/Game/Characters/Monster/UI/ThreatMeter_Widget` (`WidgetComponent.GetUserWidgetObject` (`self.ThreatMeter`))))
  (`/Game/Characters/Monster/UI/ThreatMeter_Widget.SetPercent` _asthreat_meter_widget (`self.ThreatLevel`)))

(event `LowerThreatLevel`
  (params (Value :type "Float (double-precision)"))
  ;[1 1 1] Alter Threat Level
  (bind _output_get (set `self.ThreatLevel` (- (`self.ThreatLevel`) Value)))
  (set `self.ThreatLevel` (`KismetMathLibrary.FClamp` _output_get)))

(event `ResetLostPlayer`
  ;[1 1 1] Reduce threat level
  (goto _label :!via `Reset`))

(event `SetHealth`
  ;[1 1 1] Set health value in ui
  (bind _asmonster_health_widget (cast `/Game/Characters/Monster/UI/MonsterHealth_Widget` (`WidgetComponent.GetUserWidgetObject` (`self.MonsterHealth`))))
  (`/Game/Characters/Monster/UI/MonsterHealth_Widget.SetHealth` _asmonster_health_widget (`self.Health`)))

(event `self.PawnSensing.OnHearNoise`
  (params (Instigator :type "Pawn Object Reference") (Location :type "Vector Structure (by ref)") (Volume :type "Float (single-precision)"))
  ;[1 1 1] Raise threat level on noise heard
  (switch `/Game/Characters/Monster/AI/Monster_AI_State` (`self.Monster_AI_State`)
    (:`NewEnumerator0`
      _)
    (:`NewEnumerator1`
      _)
    (:`NewEnumerator2`
      _)
    (:`NewEnumerator3`
      _)
    (:`NewEnumerator4`
      _))
  (bind _asfirst_person_character (cast `/Game/FirstPersonBP/Blueprints/FirstPersonCharacter` Instigator))
  (bind _output_get (set `self.Player` _asfirst_person_character))
  (set `self.PlayerVector` (`self.K2_GetActorLocation` _output_get))
  (`self.RaiseThreatLevel` 0.25)
  (set `self.Monster_AI_State` "NewEnumerator1")
  (if (== (`self.ThreatLevel`) 0.0)
    (set `self.Evasion` 10)
    (set `self.Monster_AI_State` "NewEnumerator2")))

(event `SetSpeedPerState`
  (bind _charactermovement (`self.CharacterMovement`))
  ;[1 1 1] Set speed per state
  (switch `/Game/Characters/Monster/AI/Monster_AI_State` (`self.Monster_AI_State`)
    (:`NewEnumerator1`
      (set `CharacterMovementComponent.MaxWalkSpeed` 250.0 _charactermovement :!label _label_2))
    (:`NewEnumerator2`
      (set `CharacterMovementComponent.MaxWalkSpeed` 400.0 _charactermovement))
    (:`NewEnumerator4`
      (goto _label_2))
    (:`NewEnumerator5`
      (set `CharacterMovementComponent.MaxWalkSpeed` 0.0 _charactermovement))))

(event `SetThreatMeterVisibility`
  (bind _threatmeter (`self.ThreatMeter`))
  ;[1 1 1] Threat meter visiblility
  (if (> (`self.ThreatLevel`) 0.0)
    (`SceneComponent.SetHiddenInGame` _threatmeter false false)
    (else
      (`SceneComponent.SetHiddenInGame` _threatmeter true false))))

(event `CheckPlayerDist`
  (bind _monster_ai_state (`self.Monster_AI_State`))
  (bind _player (`self.Player`))
  ;[1 1 1] Check player in range
  (if (`KismetSystemLibrary.IsValid` _player)
    (if (< (`KismetMathLibrary.VSize` (- (`self.K2_GetActorLocation` _player) (`self.K2_GetActorLocation`))) 300.0)
      (set `self.PlayerInAttackRange` true)
      (switch `/Game/Characters/Monster/AI/Monster_AI_State` _monster_ai_state
        (:`NewEnumerator2`
          (set `self.Monster_AI_State` "NewEnumerator3")
          (bind _asmonster_anim_bp (cast `/Game/Characters/Monster/Animations/Monster_AnimBP` (`SkeletalMeshComponent.GetAnimInstance` (`self.Mesh`))))
          (set `/Game/Characters/Monster/Animations/Monster_AnimBP.Attack` true _asmonster_anim_bp)))
      (else
        (set `self.PlayerInAttackRange` false)
        (switch `/Game/Characters/Monster/AI/Monster_AI_State` _monster_ai_state
          (:`NewEnumerator2`
            _)
          (:`NewEnumerator3`
            _))
        (set `self.Monster_AI_State` "NewEnumerator2")
        (bind _asmonster_anim_bp_2 (cast `/Game/Characters/Monster/Animations/Monster_AnimBP` (`SkeletalMeshComponent.GetAnimInstance` (`self.Mesh`))))
        (set `/Game/Characters/Monster/Animations/Monster_AnimBP.Attack` false _asmonster_anim_bp_2)))))

(event `DoDamageEvents`
  ;[1 1 1] Damage events
  (`/Engine/EditorBlueprintResources/StandardMacros.DoOnce` false :!label _label_3
    (:`Completed`
      (bind _output_get (set `self.Health` (- (`self.Health`) 0.07)))
      (set `self.Health` (`KismetMathLibrary.FClamp` _output_get))
      (set `self.Monster_AI_State` "NewEnumerator5")
      (bind _asmonster_anim_bp (cast `/Game/Characters/Monster/Animations/Monster_AnimBP` (`SkeletalMeshComponent.GetAnimInstance` (`self.Mesh`))))
      (set `/Game/Characters/Monster/Animations/Monster_AnimBP.MonsterHit` true _asmonster_anim_bp)
      (`KismetSystemLibrary.Delay` 0.2)
      (`self.ResetDamageEvents`))))

(event `ResetDamageEvents`
  ;[1 1 1] Damage events
  (goto _label_3 :!via `Reset`))

(event `MonsterDeathEvent`
  ;[1 1 1] Monster death event
  (if (== (`self.Health`) 0.0)
    (`/Engine/EditorBlueprintResources/StandardMacros.DoOnce` false
      (:`Completed`
        (`PrimitiveComponent.SetSimulatePhysics` (`self.Mesh`) true)
        (`SceneComponent.SetVisibility` (`self.ThreatMeter`) false false)
        (`SceneComponent.SetVisibility` (`self.MonsterHealth`) false false)
        (`KismetSystemLibrary.Delay` 3.0)
        (`self.K2_DestroyActor`)))))

(event `CheckPlayerHealth`
  (bind _player (`self.Player`))
  ;[1 1 1] Stop attacking if monster or player is dead
  (if (`KismetSystemLibrary.IsValid` _player)
    (if (not (and (> (`/Game/FirstPersonBP/Blueprints/FirstPersonCharacter.Health` _player) 0.0) (> (`self.Health`) 0.0)))
      (set `self.Monster_AI_State` "NewEnumerator0")
      (bind _asmonster_anim_bp (cast `/Game/Characters/Monster/Animations/Monster_AnimBP` (`SkeletalMeshComponent.GetAnimInstance` (`self.Mesh`))))
      (set `/Game/Characters/Monster/Animations/Monster_AnimBP.Attack` false _asmonster_anim_bp))))

(fn `UserConstructionScript`)